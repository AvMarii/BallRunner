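; Level exit volume that advances the game to the next level once every crystal has been collected.
; On any box overlap it checks for remaining BP_Crystal01 actors and prints a Polish warning if any exist.
; Otherwise it finds the current level in the TablicaLvlNames array and opens the following entry, or prints a last-level message at the end.
; A camera fade and delay are present but unconnected.
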(event `self.Box.OnComponentBeginOverlap`
  (params (OverlappedComponent :type "PrimitiveComponent Object Reference") (OtherActor :type "Actor Object Reference") (OtherComp :type "PrimitiveComponent Object Reference") (OtherBodyIndex :type Integer) (bFromSweep :type Boolean) (SweepResult :type "HitResult Structure (by ref)"))
  (bind _outactors (`GameplayStatics.GetAllActorsOfClass` "/Game/Blueprints/BP_Crystal01.BP_Crystal01_C"))
  (if (> (`KismetArrayLibrary.Array_Length` _outactors) 0)
    (`KismetSystemLibrary.PrintString` "Nie zebrano wszystkich diamentów")
    (else
      (`self.complete_lvl`))))

(fn `complete_lvl`
  (if (`self.final_lvl_index`)
    (`KismetSystemLibrary.PrintString` "Ostatni poziom")
    (else
      (`self.load_next_lvl_index`))))

(fn `final_lvl_index`
  (returns (ReturnValue :type Boolean))
  (return (== (`KismetArrayLibrary.Array_LastIndex` (`self.tablica_lvl_names`)) (`self.get_current_lvl_index`))))

(fn `get_current_lvl_index`
  (returns (ReturnValue :type Integer))
  (bind _returnvalue (`GameplayStatics.GetCurrentLevelName` true))
  (return (`KismetArrayLibrary.Array_Find` (`self.tablica_lvl_names`) _returnvalue)))

(fn `get_next_lvl_index`
  (returns (`next lvl name` :type String))
  (return (`|GetArrayItem` (`self.tablica_lvl_names`) (+ (`self.get_current_lvl_index`) 1))))

(fn `load_next_lvl_index`
  (bind _next_lvl_name (`self.get_next_lvl_index`))
  (`GameplayStatics.OpenLevel` (`KismetStringLibrary.Conv_StringToName` _next_lvl_name)))

(fn `UserConstructionScript`)