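; BP_Ball01 is a player-controlled rolling ball that can jump and restarts the level when damaged.
; Movement axes apply scaled torque to the Sphere, and Space adds an upward impulse if CanJump is set, a flag the jump never clears.
; BeginPlay fades the camera in with a sound.
; Any damage plays another sound, fades out, then reloads the current level after a delay.
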(event `InputAxis|MoveForwardBack`
  (params (AxisValue :type "Float (single-precision)"))
  (bind _str_multiply (`self.Str multiply`))
  (`PrimitiveComponent.AddTorqueInRadians` (`self.Sphere`) (`KismetMathLibrary.MakeVector` (* (stale `InputAxis|MoveLeftRight` AxisValue) _str_multiply) (* AxisValue _str_multiply)) "None" true :!label _label))

(event `InputAxis|MoveLeftRight`
  (params (AxisValue :type "Float (single-precision)"))
  (goto _label))

(event `Key|SpaceBar`
  (params (Key :type "Key Structure"))
  (:`Pressed`
    (if (`self.CanJump`)
      (set `self.CanJump` true)
      (`PrimitiveComponent.AddImpulse` (`self.Sphere`) (0.0 0.0 500.0) "None" true))))

(event `self.ReceiveBeginPlay`
  (`PlayerCameraManager.StartCameraFade` :`self` (`GameplayStatics.GetPlayerCameraManager` 0) :`Duration` 4.0 :`bHoldWhenFinished` true)
  (`GameplayStatics.PlaySound2D` "/Game/sound/Nagrywanie.Nagrywanie" 1.0 1.0 0.0 null null))

(event `self.ReceiveAnyDamage`
  (params (Damage :type "Float (single-precision)") (DamageType :type "DamageType Object Reference") (InstigatedBy :type "Controller Object Reference") (DamageCauser :type "Actor Object Reference"))
  (`GameplayStatics.PlaySound2D` "/Game/sound/Nagrywanie__2_.Nagrywanie__2_" 1.0 1.0 0.0 null null)
  (`PlayerCameraManager.StartCameraFade` :`self` (`GameplayStatics.GetPlayerCameraManager` 0) :`ToAlpha` 1.0 :`Duration` 4.0 :`bHoldWhenFinished` true)
  (`KismetSystemLibrary.Delay` 4.0)
  (bind _returnvalue (`GameplayStatics.GetCurrentLevelName` true))
  (`GameplayStatics.OpenLevel` (`KismetStringLibrary.Conv_StringToName` _returnvalue)))

(fn `UserConstructionScript`)